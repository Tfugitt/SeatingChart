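; BP_Cable is a simple level-dressing Blueprint that lets level designers place cables by editing a spline.
; Its construction script adds one spline mesh component per segment between neighboring spline points, each using the Staticmesh variable as its mesh.
; Each piece takes its start and end positions and tangents from the spline in local space, so the mesh bends along the curve.
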(fn ConstructionScript
  (bind _spline (Variables|Default|GetSpline))
  ;[0.7031 1 0.7048] This is a very simple setup using the spline mesh component and a spline, that the level designer can edit to add some cables to the level.
  (for _index (range 0 (- (Spline|GetNumberOfSplinePoints (Variables|Default|GetSpline)) 2))
    (bind _returnvalue (AddComponent|AddSplineMeshComponent false))
    (Components|StaticMesh|SetStaticMesh _returnvalue (Variables|Default|GetStaticmesh))
    (SplineMesh|SetStartandEnd _returnvalue (.Location (Spline|GetLocationandTangentatSplinePoint _spline _index "Local")) (.Tangent (Spline|GetLocationandTangentatSplinePoint _spline _index "Local")) (.Location (Spline|GetLocationandTangentatSplinePoint _spline (+ _index 1) "Local")) (.Tangent (Spline|GetLocationandTangentatSplinePoint _spline (+ _index 1) "Local")) true :!class /Script/Engine.SplineMeshComponent)))