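; Interactable button that the player character (BP_Bot) presses with an IK-assisted reach.
; A sphere overlap caches the bot and starts BPInteractionComponent's facing check, whose dispatchers toggle the hint text and trigger the press.
; Pressing plays a montage on the bot, then after a short sync delay a timeline moves the button and drives its dynamic material's emissive.
; The component receives the IK target location on BeginPlay.
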(event OnComponentBeginOverlap(InteractionArea)
  (params (OverlappedComponent :type Primitive%20Component%20Object%20Reference) (OtherActor :type Actor%20Object%20Reference) (OtherComp :type Primitive%20Component%20Object%20Reference) (OtherBodyIndex :type Integer) (bFromSweep :type Boolean) (SweepResult :type Hit%20Result%20Structure%20%28by%20ref%29))
  ;[1 0.6214 0.9068] The interaction area is a sphere with a custom collision. It only overlaps with a pawn. When it does, we start the check if the character is roughly facing this actor. We cast here to the BP_Bot to play the anim montage on him when the button get's pressed. This is a hard reference so when this blueprint is loaded it will also load the BP_Bot which will load more references. You can use soft references or try to avoid casting like this. This button is only ever loaded when BP_Bot is already in memory, but if you were to move it to the main menu level you would increase loading times and memory usages.
  (Default|StartCharacterOrientationCheck (Variables|Default|GetBP_InteractionComponent))
  (bind _asbp_bot (Utilities|Casting|CastToBP_Bot OtherActor))
  (Variables|Default|SetInteractingCharacter _asbp_bot))

(event OnComponentEndOverlap(InteractionArea)
  (params (OverlappedComponent :type Primitive%20Component%20Object%20Reference) (OtherActor :type Actor%20Object%20Reference) (OtherComp :type Primitive%20Component%20Object%20Reference) (OtherBodyIndex :type Integer))
  ;[0.5713 1 0.6743] When the character ends overlapping, stop the orientation check and clear the Interacting Character reference.
  (Default|EndCharacterOrientationCheck (Variables|Default|GetBP_InteractionComponent))
  (Variables|Default|SetInteractingCharacter 0))

(event Custom|OnInteract
  (params (On :type Boolean))
  ;[0.4859 0.6186 1] Assign an event to the event dispatcher so when the player presses INTERACT the button gets pressed.
  (CallFunction|PressButton))

(event Custom|OnToggleInteraction
  (params (On :type Boolean))
  ;[0.4859 0.6186 1] Assign an event to the event dispatcher so when the interaction is possible show the widget component with the hint text
  (Rendering|SetVisibility (Variables|Default|GetHintText) On false))

(event Custom|PressButton
  ;[0.5993 1 0.9781 1 12] Tell the character to play the montage pressing the button. That is in an upper body slot and has a curve that drives how much and when to blend into IK so he really reached for the button
  (Animation|PlayAnimMontage (Variables|Default|GetInteractingCharacter) "/Game/Assets/Characters/Bot/Animations/AM_Bot_Interact_PressButton.AM_Bot_Interact_PressButton" 1.0 "None")
  ;[0.5993 1 0.9781 1 12] We wait a bit before the button begins to move to sync the button movement and the animation.
  (Utilities|FlowControl|Delay 0.2)
  ;[0.5993 1 0.9781 1 12] Using a timeline to move the button and change it's emissive. In construction script we created the dynamic material and saved the reference.
  (bind _buttonmovement (Timeline|ButtonAnimation PlayFromStart)
    (:Update
      (Transformation|SetRelativeLocation (Variables|Default|GetButton) (Math|Vector|MakeVector 0.0 0.0 (* _buttonmovement -1e+01)) false false)
      (Rendering|Material|SetScalarParameterValue (Variables|Default|GetMat) "Emissive" (* _buttonmovement 5.0) :!class /Script/Engine.MaterialInstanceDynamic))))

(event EventBeginPlay
  ;[0.4859 0.6186 1] Assign an event to the event dispatcher so when the player presses INTERACT the button gets pressed.
  (EventDispatchers|AssignOnInteract (Variables|Default|GetBP_InteractionComponent) (delegate Custom|OnInteract))
  ;[0.4859 0.6186 1] Assign an event to the event dispatcher so when the interaction is possible show the widget component with the hint text
  (EventDispatchers|AssignOnToggleInteractability (Variables|Default|GetBP_InteractionComponent) (delegate Custom|OnToggleInteraction))
  ;[1 0.6995 0.6455] Save the interaction location to the interaction component. The animation BP will take that data and feed it into the control rig so the character blends into IK when they press the button.
  (Variables|/Game/Assets/Blueprints/Abilities/BP_InteractionComponent.BP_InteractionComponent_C|SetInteractionWorldLocation (Variables|Default|GetBP_InteractionComponent) (Transformation|GetWorldLocation (Variables|Default|GetIKLocation))))

(fn ConstructionScript
  (bind _returnvalue (Rendering|Material|CreateDynamicMaterialInstance (Variables|Default|GetButton) 0 "/Game/Assets/Environment/Materials/MI_Glow.MI_Glow" "None" :!class /Script/Engine.PrimitiveComponent))
  (bind _output_get (Variables|Default|SetMat _returnvalue))
  (Rendering|Material|SetScalarParameterValue _output_get "Emissive" 0.0 :!class /Script/Engine.MaterialInstanceDynamic))