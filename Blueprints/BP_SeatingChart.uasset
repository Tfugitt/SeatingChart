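; Seating chart puzzle actor that assigns named people to three rows on BeginPlay, then calls CheckResults.
; Each row function gates three hardcoded names behind one condition: YearsWorked for row 1, Charlie's name length for row 2, DaveYears for row 3.
; A trigger volume deactivates the chart when a BP_Bot leaves; its begin overlap only casts.
; AlphaName is an empty stub.
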(event OnActorBeginOverlap(TriggerVolume)
  (params (OverlappedActor :type Actor%20Object%20Reference) (OtherActor :type Actor%20Object%20Reference))
  (Utilities|Casting|CastToBP_Bot OtherActor))

(event OnActorEndOverlap(TriggerVolume)
  (params (OverlappedActor :type Actor%20Object%20Reference) (OtherActor :type Actor%20Object%20Reference))
  (Utilities|Casting|CastToBP_Bot OtherActor)
  (CallFunction|DeactivateSeatingChart))

(event EventBeginPlay
  (CallFunction|LessThan3Row)
  (CallFunction|RowbyName)
  (CallFunction|Greaterthan8Row)
  (CallFunction|CheckResults))

(fn ConstructionScript)

(fn AlphaName)

(fn LessThan3Row
  (if (< (Variables|Default|GetYearsWorked) 3)
    (CallFunction|AddNametoRow (Variables|Default|GetAnna) 1)
    (CallFunction|AddNametoRow (Variables|Default|GetBill) 1)
    (CallFunction|AddNametoRow (Variables|Default|GetIan) 1)))

(fn RowbyName
  (if (>= (Utilities|String|Len (Variables|Default|GetCharlie)) 7)
    (CallFunction|AddNametoRow (Variables|Default|GetCharlie) 2)
    (CallFunction|AddNametoRow (Variables|Default|GetGermaine) 2)
    (CallFunction|AddNametoRow (Variables|Default|GetHarmony) 2)))

(fn Greaterthan8Row
  (if (> (Variables|Default|GetDaveYears) 8)
    (CallFunction|AddNametoRow (Variables|Default|GetDave) 3)
    (CallFunction|AddNametoRow (Variables|Default|GetEileen) 3)
    (CallFunction|AddNametoRow (Variables|Default|GetFrank) 3)))