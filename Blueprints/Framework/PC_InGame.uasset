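; In-game player controller that clamps camera pitch, sets game-only input and handles non-pawn input such as pausing.
; It creates and owns the heads-up display widget, while pause requests are passed to the HUD as a toggle of the paused state.
; An AnyKey listener detects gamepad versus keyboard input to switch control hints, a Blueprint-only workaround.
; F9 also triggers pause outside distribution builds, since Escape closes play-in-editor.
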(event Input|EnhancedActionEvents|EnhancedInputActionIA_Pause
  (params (ActionValue :type Boolean) (ElapsedSeconds :type Float%20%28double-precision%29) (TriggeredSeconds :type Float%20%28double-precision%29) (InputAction :type Input%20Action%20Object%20Reference :default "/Game/Assets/Input/IA_Pause.IA_Pause"))
  ;[0.3832 0.9901 1] Key Binding (Pause Menu)
  ; You will notice we will have input proccessed here in the player controller and in the BP_Bot character.
  ; In this projects case that is fine. The player controller handles everything expect the pawn controls.
  ; In a project where you might have several different characters you control, you might want to have all input in the controller and and the pawn/character executing them. Also for multiplayer this setup is not sufficient.
  ; Think of the controller being the brain and the pawn being the body executing the brains commands.
  ; That said we made the conscious decision to keep the input for the character in BP_Bot
  (:Triggered
    (Class|BPIHUDInterface|SetPaused(Message) (HUD|GetHUD) (not (Game|IsGamePaused)))))

(event EventBeginPlay
  (bind _playercameramanager (Variables|Default|GetPlayerCameraManager))
  (Utilities|FlowControl|Sequence
    (:then_0
      ;[0.7469 1 0.4938] The player controller also has a reference to the camera manager. We set the min and max to clamp the pitch
      (Variables|/Script/Engine.PlayerCameraManager|SetViewPitchMin _playercameramanager -65.0)
      (Variables|/Script/Engine.PlayerCameraManager|SetViewPitchMax _playercameramanager 0.0))
    (:then_1
      ;[0.7047 0.7262 1] Change input mode and hide mouse cursor
      (Input|SetInputModeGameOnly self false)
      (Variables|Default|SetbShowMouseCursor false))
    (:then_2
      ;[1 0.523 0.5648] While the pause menu is spawned and handled by the HUD_InGame this player controler owns the head up display where we show the amount of orbs, when the game is saved and controller hints.
      (bind _returnvalue (UserInterface|CreateWidget "/Game/Assets/Blueprints/UI/BPW_HeadupDisplay.BPW_HeadupDisplay_C" self))
      (bind _output_get (Variables|Default|SetHeadupDisplay _returnvalue))
      (UserInterface|Viewport|AddtoViewport _output_get 0))))

(event Input|KeyboardEvents|F9
  (params (Key :type Key%20Structure))
  ;[0.5434 0.8604 1 1 12] F5 only in editor not packaged build as Escape closed play in editor.
  (:Pressed
    (if (not (Class|KismetSystemLibrary|IsPackagedforDistribution))
      ;[0.3832 0.9901 1] Key Binding (Pause Menu)
      ; You will notice we will have input proccessed here in the player controller and in the BP_Bot character.
      ; In this projects case that is fine. The player controller handles everything expect the pawn controls.
      ; In a project where you might have several different characters you control, you might want to have all input in the controller and and the pawn/character executing them. Also for multiplayer this setup is not sufficient.
      ; Think of the controller being the brain and the pawn being the body executing the brains commands.
      ; That said we made the conscious decision to keep the input for the character in BP_Bot
      (Class|BPIHUDInterface|SetPaused(Message) (HUD|GetHUD) (not (Game|IsGamePaused))))))

(event Input|KeyboardEvents|AnyKey
  (params (Key :type Key%20Structure))
  (bind _returnvalue (Class|KismetInputLibrary|KeyIsGamepadKey Key))
  ;[0.5071 0.9661 1] Proper gamepad and keyboard/mouse support you usually need some C++.
  ; This is more a workaround as this is a BP only project.
  ; When any key is pressed we check if it is coming from a  gamepad. In this way we can toggle between keyboard/ mouse and gamepad input hints. In this case in the headup widget we show the key or the gamepad button to press. In a bigger project this will not hold up. Especially on startup or reloading the map, you can not easily know what the last input device was.
  ; Important to know that this event doesnt consume the input.
  (:Pressed
    (Default|ToggleControlDisplay (Variables|/Game/Assets/Blueprints/UI/BPW_HeadupDisplay.BPW_HeadupDisplay_C|GetBPW_Controls (Variables|Default|GetHeadupDisplay)) _returnvalue)
    (Variables|Default|SetIsUsingGamepad _returnvalue)))

(fn ConstructionScript)