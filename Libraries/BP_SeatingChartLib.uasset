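; Blueprint function library for a seating chart exercise where names are added to three rows and checked against a fixed answer.
; AddNameToRow finds or creates the UI_SeatingChart widget, then appends the name to the chosen row as comma-separated text.
; CheckResults compares each row's exact text, so order matters, marking wrong rows Incorrect and showing Success in the repurposed fourth row.
; DeactivateSeatingChart removes all widgets.
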(fn AddNametoRow
  (params (Name :type String) (Row :type Integer))
  (LocalVariables|Set_Name Name)
  (bind __seatingchart (CallFunction|SetupSeatingChart (LocalVariables|Get__WorldContext)))
  (LocalVariables|SetSeatingChart __seatingchart)
  (switch int Row
    (:1
      (CallFunction|AppendRowText (LocalVariables|Get__WorldContext) (Variables|/Game/Libraries/UI_SeatingChart.UI_SeatingChart_C|Gettxt_RowOne (LocalVariables|GetSeatingChart)) (LocalVariables|Get_Name)))
    (:2
      (CallFunction|AppendRowText (LocalVariables|Get__WorldContext) (Variables|/Game/Libraries/UI_SeatingChart.UI_SeatingChart_C|Gettxt_RowTwo (LocalVariables|GetSeatingChart)) (LocalVariables|Get_Name)))
    (:3
      (CallFunction|AppendRowText (LocalVariables|Get__WorldContext) (Variables|/Game/Libraries/UI_SeatingChart.UI_SeatingChart_C|Gettxt_RowThree (LocalVariables|GetSeatingChart)) (LocalVariables|Get_Name)))
    (:4)))

(fn SetupSeatingChart
  (bind _foundwidgets (Widget|GetAllWidgetsOfClass (LocalVariables|Get__WorldContext) "/Game/Libraries/UI_SeatingChart.UI_SeatingChart_C"))
  (if (> (Utilities|Array|Length _foundwidgets) 0)
    (LocalVariables|Set__SeatingChart (Utilities|Array|Get(acopy) _foundwidgets))
    (else
      (bind _returnvalue (UserInterface|CreateWidget "/Game/Libraries/UI_SeatingChart.UI_SeatingChart_C" (Class|GameplayStatics|GetPlayerControllerfromID (LocalVariables|Get__WorldContext))))
      (bind _output_get (LocalVariables|Set__SeatingChart _returnvalue))
      (UserInterface|Viewport|AddtoViewport _output_get 0)
      (CallFunction|ClearText (LocalVariables|Get__SeatingChart) (LocalVariables|Get__WorldContext))))
  (return (LocalVariables|Get__SeatingChart)))

(fn ClearText
  (params (SeatingChart :type UI%20Seating%20Chart%20Object%20Reference))
  (Rendering|Components|TextRender|SetText (Variables|/Game/Libraries/UI_SeatingChart.UI_SeatingChart_C|Gettxt_RowOne SeatingChart) "Row 1:")
  (Rendering|Components|TextRender|SetText (Variables|/Game/Libraries/UI_SeatingChart.UI_SeatingChart_C|Gettxt_RowTwo SeatingChart) "Row 2:")
  (Rendering|Components|TextRender|SetText (Variables|/Game/Libraries/UI_SeatingChart.UI_SeatingChart_C|Gettxt_RowThree SeatingChart) "Row 3:")
  ;[1 1 1] Repurposed row 4 for "success."
  (Rendering|Components|TextRender|SetText (Variables|/Game/Libraries/UI_SeatingChart.UI_SeatingChart_C|Gettxt_RowFour SeatingChart) ""))

(fn AppendRowText
  (params (Row :type Text%20Block%20Object%20Reference) (Name :type String))
  (LocalVariables|Set_Row Row)
  (LocalVariables|Set_Name Name)
  (if (< (Utilities|String|Len (Utilities|String|ToString(Text) (Class|TextBlock|GetText (LocalVariables|Get_Row)))) 7)
    (Rendering|Components|TextRender|SetText (LocalVariables|Get_Row) (Utilities|Text|FormatText "{existingValue} {name}" (Class|TextBlock|GetText (LocalVariables|Get_Row)) (LocalVariables|Get_Name)))
    (else
      (Rendering|Components|TextRender|SetText (LocalVariables|Get_Row) (Utilities|Text|FormatText "{existingValue}, {name}" (Class|TextBlock|GetText (LocalVariables|Get_Row)) (LocalVariables|Get_Name))))))

(fn CheckResults
  (bind _foundwidgets (Widget|GetAllWidgetsOfClass (LocalVariables|Get__WorldContext) "/Game/Libraries/UI_SeatingChart.UI_SeatingChart_C"))
  (if (> (Utilities|Array|Length _foundwidgets) 0)
    (if (Utilities|Enum|Equal(Enum) (Class|TextBlock|GetText (Variables|/Game/Libraries/UI_SeatingChart.UI_SeatingChart_C|Gettxt_RowOne (Utilities|Array|Get(acopy) _foundwidgets))) (Utilities|Text|MakeLiteralText "Row 1: Anna, Bill, Ian"))
      (Math|Integer|IncrementInt (LocalVariables|GetCorrectCount)
        (:%20%20
          _))
      (else
        (Rendering|Components|TextRender|SetText (Variables|/Game/Libraries/UI_SeatingChart.UI_SeatingChart_C|Gettxt_RowOne (Utilities|Array|Get(acopy) _foundwidgets)) (Utilities|Text|FormatText "{value} — Incorrect" (Class|TextBlock|GetText (Variables|/Game/Libraries/UI_SeatingChart.UI_SeatingChart_C|Gettxt_RowOne (Utilities|Array|Get(acopy) _foundwidgets)))))))
    (if (Utilities|Enum|Equal(Enum) (Class|TextBlock|GetText (Variables|/Game/Libraries/UI_SeatingChart.UI_SeatingChart_C|Gettxt_RowTwo (Utilities|Array|Get(acopy) _foundwidgets))) (Utilities|Text|MakeLiteralText "Row 2: Charlie, Germaine, Harmony"))
      (Math|Integer|IncrementInt (LocalVariables|GetCorrectCount)
        (:%20%20
          _))
      (else
        (Rendering|Components|TextRender|SetText (Variables|/Game/Libraries/UI_SeatingChart.UI_SeatingChart_C|Gettxt_RowTwo (Utilities|Array|Get(acopy) _foundwidgets)) (Utilities|Text|FormatText "{value} — Incorrect" (Class|TextBlock|GetText (Variables|/Game/Libraries/UI_SeatingChart.UI_SeatingChart_C|Gettxt_RowTwo (Utilities|Array|Get(acopy) _foundwidgets)))))))
    (if (Utilities|Enum|Equal(Enum) (Class|TextBlock|GetText (Variables|/Game/Libraries/UI_SeatingChart.UI_SeatingChart_C|Gettxt_RowThree (Utilities|Array|Get(acopy) _foundwidgets))) (Utilities|Text|MakeLiteralText "Row 3: Dave, Eileen, Frank"))
      (Math|Integer|IncrementInt (LocalVariables|GetCorrectCount)
        (:%20%20
          _))
      (else
        (Rendering|Components|TextRender|SetText (Variables|/Game/Libraries/UI_SeatingChart.UI_SeatingChart_C|Gettxt_RowThree (Utilities|Array|Get(acopy) _foundwidgets)) (Utilities|Text|FormatText "{value} — Incorrect" (Class|TextBlock|GetText (Variables|/Game/Libraries/UI_SeatingChart.UI_SeatingChart_C|Gettxt_RowThree (Utilities|Array|Get(acopy) _foundwidgets)))))))
    (if (== (LocalVariables|GetCorrectCount) 3)
      (Rendering|Components|TextRender|SetText (Variables|/Game/Libraries/UI_SeatingChart.UI_SeatingChart_C|Gettxt_RowFour (Utilities|Array|Get(acopy) _foundwidgets)) "Success!"))
    (else
      (Development|PrintString (LocalVariables|Get__WorldContext) "Something went wrong.  Have you called AddNameToRow anywhere?" true true "(R=1.000000,G=0.000000,B=0.000000,A=1.000000)"))))

(fn DeactivateSeatingChart
  (Viewport|RemoveAllWidgets (LocalVariables|Get__WorldContext))
  (Utilities|Platform|CollectGarbage))